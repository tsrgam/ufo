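; BP_Tree is a placeable tree actor that varies its mesh, uniform scale, yaw and color bias per instance.
; The Construction Script derives a deterministic seed from world location using a dot product and modulo, so variation follows placement.
; That seed drives all four properties, with color bias passed to the material through Custom Primitive Data.
; LockRandomness skips recomputation, keeping the current values when the tree moves.
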(fn `UserConstructionScript`
  (if (not (`self.LockRandomness`))
    (set `self.RandomSeed` (`KismetMathLibrary.Abs_Int` (mod (`KismetMathLibrary.FTrunc` (`KismetMathLibrary.Dot_VectorVector` (.location (`SceneComponent.K2_GetComponentToWorld` (`self.Tree`))) (`self.RandomVariable012`))) (`self.RandomVariable3`))))
    (set `self.TreeIndex` (mod (`self.RandomSeed`) (`KismetArrayLibrary.Array_Length` (`self.TreeMeshes`))))
    (set `self.ScaleModifier` (`KismetMathLibrary.Lerp` (`self.RandomScaleMin`) (`self.RandomScaleMax`) (/ (`KismetMathLibrary.Conv_IntToDouble` (`self.RandomSeed`)) (`KismetMathLibrary.Conv_IntToDouble` (`self.RandomVariable3`)))))
    (set `self.RotationModifier` (`KismetMathLibrary.Conv_IntToDouble` (`self.RandomSeed`)))
    (set `self.ColorBias` (`KismetMathLibrary.Lerp` (`self.RandomColorBiasMin`) (`self.RandomColorBiasMax`) (/ (`KismetMathLibrary.Conv_IntToDouble` (`self.RandomSeed`)) (`KismetMathLibrary.Conv_IntToDouble` (`self.RandomVariable3`))))))
  (`|ExecutionSequence`
    (:`then_0`
      (`StaticMeshComponent.SetStaticMesh` (`self.Tree`) (`|GetArrayItem` (`self.TreeMeshes`) (`self.TreeIndex`)))
      (`SceneComponent.SetRelativeScale3D` (`self.Tree`) (`KismetMathLibrary.Conv_DoubleToVector` (`self.ScaleModifier`)))
      (`SceneComponent.K2_SetRelativeRotation` (`self.Tree`) (`KismetMathLibrary.MakeRotator` 0.0 0.0 (`self.RotationModifier`)) false false)
      (`PrimitiveComponent.SetCustomPrimitiveDataFloat` (`self.Tree`) (`self.CustomDataIndex_ColorBias`) (`self.ColorBias`)))))