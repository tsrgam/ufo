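; Hover component that procedurally animates a UFO from its owner's horizontal velocity every tick.
; TickTilt pitches and rolls the saucer root along the movement direction, easing up to a maximum angle with a smoothstep of speed.
; TickIdle bobs the full UFO root vertically at or below an idle speed threshold, applying sine-wave deltas as local offsets rather than setting absolute height.
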(event `self.ReceiveTick`
  (params (DeltaSeconds :type "Float (single-precision)"))
  (bind _returnvalue (`KismetMathLibrary.Conv_VectorToVector2D` (`Actor.GetVelocity` (`self.GetOwner`))))
  (bind _returnvalue_2 (`KismetMathLibrary.VSize2D` _returnvalue))
  (`self.TickTilt` (`KismetMathLibrary.Normal2D` _returnvalue) _returnvalue_2)
  (`self.TickIdle` DeltaSeconds _returnvalue_2))

(fn `TickIdle`
  (params (DeltaSeconds :type "Float (double-precision)") (MoveSpeed :type "Float (double-precision)"))
  (bind _returnvalue (`KismetMathLibrary.Sin` (* (`self.TimeSinceStart`) (`self.IdleBobSpeed`))))
  (if (not (> MoveSpeed (`self.IdleSpeedThreshold`)))
    (set `self.TimeSinceStart` (+ DeltaSeconds (`self.TimeSinceStart`)))
    (`self.K2_AddLocalOffset` (`self.FullUfoRoot`) (`KismetMathLibrary.MakeVector` 0.0 0.0 (* (- _returnvalue (`self.CachedYOffset`)) (`self.IdleBobAmplitude`))) false false)
    (set `self.CachedYOffset` _returnvalue)))

(fn `TickTilt`
  (params (MoveDirection :type "Vector2D Structure") (MoveSpeed :type "Float (double-precision)"))
  (bind (_x _y) (`KismetMathLibrary.BreakVector2D` (* MoveDirection (* (`self.Smoothstep` 0.0 (`self.MaxTiltSpeed`) MoveSpeed) (`self.MaxTiltAngle`)))))
  (`self.K2_SetRelativeRotation` (`self.SaucerRoot`) (`KismetMathLibrary.MakeRotator` _y (* _x -1.0)) false false))