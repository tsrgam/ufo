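; Player UFO character that moves on world axes and abducts collectables with a tractor beam while TurnOn is held.
; Pressing it shows the spotlight and locks the first actor overlapping TraceCone, disabling its gravity, spinning it and notifying its BP_CollectableComponent.
; Tick pulls the locked actor toward the UFO while shrinking it; release restores gravity and scale.
; Any actor that begins overlapping CollectionCylinder is destroyed, clearing the lock.
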(event `InputAxis|MoveNorth`
  (params (AxisValue :type "Float (single-precision)"))
  (`self.AddMovementInput` (1.0 0.0 0.0) AxisValue))

(event `InputAxis|MoveEast`
  (params (AxisValue :type "Float (single-precision)"))
  (`self.AddMovementInput` (0.0 1.0 0.0) AxisValue))

(event `InputAction|TurnOn`
  (params (Key :type "Key Structure"))
  (bind _spotligh1 (`self.SpotLigh1`))
  (bind _tracecone (`self.TraceCone`))
  (bind _lockedoncollectable (`self.LockedOnCollectable`))
  (bind _returnvalue (`self.GetComponentByClass` (`self.LockedOnCollectable`) "/Game/Blueprints/BP_CollectableComponent.BP_CollectableComponent_C"))
  (bind _returnvalue_2 (`self.GetComponentByClass` (`self.LockedOnCollectable`) "/Game/Blueprints/BP_CollectableComponent.BP_CollectableComponent_C"))
  (:`Pressed`
    (`SceneComponent.SetVisibility` _spotligh1 true false)
    (bind _outactors (`KismetSystemLibrary.ComponentOverlapActors` _tracecone (`SceneComponent.K2_GetComponentToWorld` _tracecone) (`|MakeArray` "ObjectTypeQuery7" :!type "EObjectTypeQuery Enum")))
    (if (`KismetArrayLibrary.Array_IsValidIndex` _outactors)
      (bind _output (`|GetArrayItem` _outactors))
      (set `self.LockedOnCollectable` _output)
      (bind _asprimitive_component (cast `PrimitiveComponent` (`Actor.RootComponent` _output)))
      (`PrimitiveComponent.SetSimulatePhysics` _asprimitive_component true)
      (`PrimitiveComponent.SetEnableGravity` _asprimitive_component false)
      (`PrimitiveComponent.SetCollisionProfileName` _asprimitive_component "BlockAllStatic")
      (`PrimitiveComponent.SetAllPhysicsLinearVelocity` _asprimitive_component (0.0 0.0 0.0) false)
      (`PrimitiveComponent.SetAllPhysicsAngularVelocityInDegrees` _asprimitive_component (`KismetMathLibrary.MakeVector` 50.0 50.0) false)
      (`/Engine/EditorBlueprintResources/StandardMacros.IsValid` _returnvalue_2
        (:`Is Valid`
          (`/Game/Blueprints/BP_CollectableComponent.OnTractorBeamLocked` _returnvalue_2)))))
  (:`Released`
    (`SceneComponent.SetVisibility` _spotligh1 false false)
    (`/Engine/EditorBlueprintResources/StandardMacros.IsValid` _lockedoncollectable
      (:`Is Valid`
        (bind _asprimitive_component_2 (cast `PrimitiveComponent` (`Actor.RootComponent` _lockedoncollectable))
          (:`then`
            (`PrimitiveComponent.SetEnableGravity` _asprimitive_component_2 true)
            (`PrimitiveComponent.SetAllPhysicsAngularVelocityInDegrees` _asprimitive_component_2 (`KismetMathLibrary.Vector_Zero`) false)
            (`self.SetActorRelativeScale3D` (`self.LockedOnCollectable`) (1.0 1.0 1.0))
            (`PrimitiveComponent.SetCollisionProfileName` _asprimitive_component_2 "BlockAllDynamic")
            (`/Engine/EditorBlueprintResources/StandardMacros.IsValid` _returnvalue
              (:`Is Valid`
                (`/Game/Blueprints/BP_CollectableComponent.OnTractorBeamUnlocked` _returnvalue))
              (:`Is Not Valid`
                _)))
          (:`CastFailed`
            _)))
      (:`Is Not Valid`
        _))
    (set `self.LockedOnCollectable` null)))

(event `self.ReceiveTick`
  (params (DeltaSeconds :type "Float (single-precision)"))
  (bind _lockedoncollectable (`self.LockedOnCollectable`))
  (bind _lockedoncollectable_2 (`self.LockedOnCollectable`))
  (`/Engine/EditorBlueprintResources/StandardMacros.IsValid` _lockedoncollectable_2
    (:`Is Valid`
      (`self.K2_AddActorWorldOffset` _lockedoncollectable_2 (* (`KismetMathLibrary.Normal` (- (`self.K2_GetActorLocation`) (`self.K2_GetActorLocation` _lockedoncollectable_2))) (* DeltaSeconds (`self.TransportSpeed`))) true true)
      (`/Engine/EditorBlueprintResources/StandardMacros.IsValid` _lockedoncollectable
        (:`Is Valid`
          (`self.SetActorRelativeScale3D` _lockedoncollectable (`KismetMathLibrary.Vector_ComponentMax` (- (`self.GetActorRelativeScale3D` _lockedoncollectable) (* (`self.ShrinkSpeed`) DeltaSeconds)) (0.1 0.1 0.1))))))))

(event `self.CollectionCylinder.OnComponentBeginOverlap`
  (params (OverlappedComponent :type "PrimitiveComponent Object Reference") (OtherActor :type "Actor Object Reference") (OtherComp :type "PrimitiveComponent Object Reference") (OtherBodyIndex :type Integer) (bFromSweep :type Boolean) (SweepResult :type "HitResult Structure (by ref)"))
  (`self.K2_DestroyActor` OtherActor)
  (set `self.LockedOnCollectable` null))

(fn `UserConstructionScript`)